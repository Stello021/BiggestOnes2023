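; Overworld game mode that restores defeated-enemy state and runs the Tutorial_Castle intro cutscene.
; On BeginPlay it destroys "Enemy"-tagged actors whose IDs the game instance records as killed, then, if the cutscene is unplayed, disables input and plays the level sequence.
; Tick lets Q skip the cutscene, marking it played and briefly showing a tutorial commands widget.
; A dialogue event runs the behavior tree of a randomly picked BPC_WilpAreaSpawn actor.
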(event `self.ReceiveBeginPlay`
  (bind _outactors (`GameplayStatics.GetAllActorsWithTag` "Enemy"))
  (for _array_element _outactors
    (bind _asbp_enemy (cast `/Game/Blueprints/Enemies/BP_Enemy` _array_element))
    (bind _asbp_game_instance (cast `/Game/Blueprints/GameInstances/BP_GameInstance` (`GameplayStatics.GetGameInstance`)))
    (for _array_element_2 (`/Game/Blueprints/GameInstances/BP_GameInstance.TutorialEnemiesKilledID` _asbp_game_instance)
      (if (== _array_element_2 (`/Game/Blueprints/Enemies/BP_Enemy.EnemyID` _asbp_enemy))
        (`self.K2_DestroyActor` _asbp_enemy))))
  (bind _asbp_game_instance_2 (cast `/Game/Blueprints/GameInstances/BP_GameInstance` (`GameplayStatics.GetGameInstance`)))
  (bind _returnvalue (`GameplayStatics.GetCurrentLevelName` true))
  (if (`KismetStringLibrary.EqualEqual_StrStr` _returnvalue "Tutorial_Castle")
    (if (not (`/Game/Blueprints/GameInstances/BP_GameInstance.IsPlayedCutScene` _asbp_game_instance_2))
      (`self.DisableInput` (`GameplayStatics.GetPlayerPawn` 0) (`GameplayStatics.GetPlayerController` 0))
      (`self.PlayCutScene`))))

(event `OnFinished_StartDialogue`
  (bind _outactors (`GameplayStatics.GetAllActorsOfClass` "/Game/Blueprints/AI/NPC_ConditionSpawn/BPC_WilpAreaSpawn.BPC_WilpAreaSpawn_C"))
  (bind _outitem (`KismetArrayLibrary.Array_Random` _outactors))
  (`AIController.RunBehaviorTree` (`AIBlueprintHelperLibrary.GetAIController` _outitem) (`/Game/Blueprints/AI/BPC_MainNPC.Dialogue Tree` _outitem)))

(event `self.ReceiveTick`
  (params (DeltaSeconds :type "Float (single-precision)"))
  (bind _output_cutscene (`self.Get CutSceneStart`))
  (`/Engine/EditorBlueprintResources/StandardMacros.IsValid` _output_cutscene
    (:`Is Valid`
      (bind _asbp_game_instance (cast `/Game/Blueprints/GameInstances/BP_GameInstance` (`GameplayStatics.GetGameInstance`)))
      (if (not (`/Game/Blueprints/GameInstances/BP_GameInstance.IsPlayedCutScene` _asbp_game_instance))
        (bind _returnvalue (`GameplayStatics.GetCurrentLevelName` true))
        (if (and (`KismetStringLibrary.EqualEqual_StrStr` _returnvalue "Tutorial_Castle") (`PlayerController.WasInputKeyJustPressed` (`GameplayStatics.GetPlayerController` 0) "Q") (`MovieSceneSequencePlayer.IsPlaying` _output_cutscene))
          (set `/Game/Blueprints/GameInstances/BP_GameInstance.IsPlayedCutScene` true _asbp_game_instance)
          (`MovieSceneSequencePlayer.GoToEndAndStop` _output_cutscene)
          (bind _returnvalue_2 (`|CreateWidget` "/Game/UI/Widgets/UI_Player/WB_TutorialComands.WB_TutorialComands_C" (`GameplayStatics.GetPlayerController` 0)))
          (`UserWidget.AddToViewport` _returnvalue_2 0)
          (`KismetSystemLibrary.Delay` 3.0)
          (`Widget.RemoveFromParent` _returnvalue_2)
          (`self.OnFinished_StartDialogue`))))))

(fn `Get CutSceneStart`
  (returns (Output_CutScene :type "LevelSequencePlayer Object Reference"))
  (return (`self.CutSceneStart`)))

(fn `PlayCutScene`
  (locals (StartCutScene :type "LevelSequencePlayer Object Reference"))
  (bind (_outactor _returnvalue) (`LevelSequencePlayer.CreateLevelSequencePlayer` "/Game/Cinematics/Sequences/Sequence/shot/shot0010/shot0010_01.shot0010_01"))
  (bind _output_get (set `local.StartCutScene` _returnvalue))
  (`self.Set CutSceneVariable` _output_get)
  (`MovieSceneSequencePlayer.Play` _output_get)
  (add `MovieSceneSequencePlayer.OnFinished` _output_get (`|CreateDelegate` :!event `OnFinished_StartDialogue`)))

(fn `Set CutSceneVariable`
  (params (NewParam :type "LevelSequencePlayer Object Reference"))
  (set `self.CutSceneStart` NewParam))

(fn `UserConstructionScript`)