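; AI controller for patrolling enemies that runs the BT_EnemyPatrol behavior tree on BeginPlay and tracks the player by sight.
; Perception updates pass to HandleSightSense, which ignores non-sight stimuli and any actor other than the first player character.
; It sets the TargetActor blackboard key while the player is seen, and clears it on lost sight while storing the stimulus location in LastKnowLocation.
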(event `self.ReceiveBeginPlay`
  (`self.RunBehaviorTree` "/Game/Blueprints/Enemy_AI/BT_EnemyPatrol.BT_EnemyPatrol"))

(event `self.AIPerception.OnTargetPerceptionUpdated`
  (params (Actor :type "Actor Object Reference") (Stimulus :type "AIStimulus Structure"))
  (`self.HandleSightSense` Actor Stimulus))

(fn `HandleSightSense`
  (params (Actor :type "Actor Object Reference") (Stimulis :type "AIStimulus Structure"))
  (bind (_stimulis_age _stimulis_expirationage _stimulis_strength _stimulis_stimuluslocation _stimulis_receiverlocation _stimulis_tag _stimulis_bsuccessfullysensed) (break `AIStimulus` (`local.Stimulis`)))
  (bind _returnvalue (`AIPerceptionSystem.GetSenseClassForStimulus` Stimulis))
  (if (== _returnvalue "/Script/AIModule.AISense_Sight")
    (if (== (`local.Actor`) (`GameplayStatics.GetPlayerCharacter` 0))
      (`BlackboardComponent.SetValueAsObject` (`self.Blackboard`) "TargetActor" (`KismetMathLibrary.SelectObject` (`GameplayStatics.GetPlayerCharacter` 0) null _stimulis_bsuccessfullysensed))
      (if (not _stimulis_bsuccessfullysensed)
        (`BlackboardComponent.SetValueAsVector` (`self.Blackboard`) "LastKnowLocation" _stimulis_stimuluslocation))
      (else
        (return)))
    (else
      (return))))

(fn `UserConstructionScript`)