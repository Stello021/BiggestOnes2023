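; BP_WallSphere is an overlap trigger that shows the player a wall message and can remove an associated wall.
; When a BP_Player begins overlapping, it creates a WB_WallMessagge widget, fills it with its TextLine text and destroys WallToDestroy if that reference is valid.
; End overlap removes the widget from the screen without checking which actor left.
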(event `self.ReceiveBeginPlay`)

(event `self.ReceiveActorBeginOverlap`
  (params (OtherActor :type "Actor Object Reference"))
  (bind _wall_to_destroy (`self.Wall To Destroy`))
  (cast `/Game/Blueprints/Player/Blueprints/BP_Player` OtherActor)
  (bind _returnvalue (`|CreateWidget` "/Game/UI/Widgets/WallCollision/WB_WallMessagge.WB_WallMessagge_C"))
  (`UserWidget.AddToViewport` _returnvalue 0)
  (set `TextBlock.Text` (`self.TextLine`) (`/Game/UI/Widgets/WallCollision/WB_WallMessagge.TB_TextLine` _returnvalue))
  (`/Engine/EditorBlueprintResources/StandardMacros.IsValid` _wall_to_destroy
    (:`Is Valid`
      (`self.K2_DestroyActor` _wall_to_destroy))))

(event `self.ReceiveActorEndOverlap`
  (params (OtherActor :type "Actor Object Reference"))
  (`Widget.RemoveFromParent` (stale `self.ReceiveActorBeginOverlap` _returnvalue)))

(fn `UserConstructionScript`)