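; BP_InvisibleWall is a trigger that shows a text message while the player overlaps it and clears a linked wall actor.
; Player overlap creates a WB_WallMessagge widget with TextLine and destroys WallToDestroy; ending any overlap removes the widget.
; The wall's OnDestroyed event records the trigger's display name in BP_GameInstance's WallIsActive array.
; On BeginPlay the trigger prints that lookup and destroys itself if already recorded.
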(event `self.ReceiveBeginPlay`
  (bind _asbp_game_instance (cast `/Game/Blueprints/GameInstances/BP_GameInstance` (`GameplayStatics.GetGameInstance`)))
  (bind _output_get (set `self.As BP Game Instance` _asbp_game_instance))
  (bind _returnvalue (`KismetArrayLibrary.Array_Find` (`/Game/Blueprints/GameInstances/BP_GameInstance.WallIsActive` _output_get) (`KismetSystemLibrary.GetDisplayName` self)))
  (`KismetSystemLibrary.PrintString` (`KismetStringLibrary.Conv_IntToString` _returnvalue))
  (if (!= _returnvalue -1)
    (`self.K2_DestroyActor`)))

(event `self.ReceiveActorBeginOverlap`
  (params (OtherActor :type "Actor Object Reference"))
  (bind _wall_to_destroy (`self.Wall To Destroy`))
  (cast `/Game/Blueprints/Player/Blueprints/BP_Player` OtherActor)
  (bind _returnvalue (`|CreateWidget` "/Game/UI/Widgets/WallCollision/WB_WallMessagge.WB_WallMessagge_C"))
  (`UserWidget.AddToViewport` _returnvalue 0)
  (set `TextBlock.Text` (`self.TextLine`) (`/Game/UI/Widgets/WallCollision/WB_WallMessagge.TB_TextLine` _returnvalue))
  (if (not (`self.Wall Is Destroyed`))
    (`/Engine/EditorBlueprintResources/StandardMacros.IsValid` _wall_to_destroy
      (:`Is Valid`
        (`self.K2_DestroyActor` _wall_to_destroy)))))

(event `self.ReceiveActorEndOverlap`
  (params (OtherActor :type "Actor Object Reference"))
  (`Widget.RemoveFromParent` (stale `self.ReceiveActorBeginOverlap` _returnvalue)))

(event `self.Wall To Destroy.OnDestroyed`
  (params (DestroyedActor :type "Actor Object Reference"))
  (set `self.Wall Is Destroyed` true)
  (`KismetArrayLibrary.Array_Add` (`/Game/Blueprints/GameInstances/BP_GameInstance.WallIsActive` (`self.As BP Game Instance`)) (`KismetSystemLibrary.GetDisplayName` self)))

(fn `UserConstructionScript`)