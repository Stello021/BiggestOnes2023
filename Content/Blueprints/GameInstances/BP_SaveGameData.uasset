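; BP_SaveGameData is the save object that stores the overworld player's transform and per-unit stats for player units.
; Unit info lives in a map keyed by unit class, and each save function writes to the slot immediately through SaveGameFile.
; Load functions apply in-memory values, restoring location directly, but current HP and combat-component level only once a unit save has set ToBeLoaded.
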(fn `LoadPlayerLocation`
  (params (OverworldPlayerCharacter :type "/Game/Blueprints/Player/Blueprints/BP_Player Object Reference"))
  (`Actor.K2_SetActorTransform` OverworldPlayerCharacter (`self.PlayerLocation`) false false))

(fn `LoadPlayerUnitInfo`
  (params (`Player Unit` :type "/Game/Blueprints/CombatSystem/BP_UnitBase Object Reference"))
  (bind ((`UnitLevel_4_1C28E04C43F6555D02D5AA8F0EAA3F77` _unitlevel) (`HPCurrent_7_81F36A114C6D33722B9930AB2557398C` _hpcurrent)) (break `/Game/Data/ST_CharacterInfo` (`BlueprintMapLibrary.Map_Find` (`self.PlayerInfo`) (`GameplayStatics.GetObjectClass` `Player Unit`))))
  (if (`self.ToBeLoaded`)
    (set `/Game/Blueprints/CombatSystem/BP_UnitBase.CurrentHP` _hpcurrent `Player Unit`)
    (set `/Game/Blueprints/CombatSystem/BP_CombatComponent.UnitLevel` _unitlevel (`/Game/Blueprints/CombatSystem/BP_UnitBase.CombatComponent` `Player Unit`))))

(fn `SaveGameFile`
  (`GameplayStatics.SaveGameToSlot` self (`self.SlotName`)))

(fn `SavePlayerLocation`
  (params (OverworldPlayerCharacter :type "/Game/Blueprints/Player/Blueprints/BP_Player Object Reference"))
  (set `self.PlayerLocation` (`Actor.GetTransform` OverworldPlayerCharacter))
  (`self.SaveGameFile`))

(fn `SavePlayerUnitInfo`
  (params (`Player Unit` :type "/Game/Blueprints/CombatSystem/BP_UnitBase Object Reference") (Info :type "/Game/Data/ST_CharacterInfo Structure"))
  (`BlueprintMapLibrary.Map_Add` (`self.PlayerInfo`) (`GameplayStatics.GetObjectClass` `Player Unit`) Info)
  (set `self.ToBeLoaded` true)
  (`self.SaveGameFile`))