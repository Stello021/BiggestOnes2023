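; BP_Move is a trigger volume that switches the view with a cubic blend when BP_Player enters and returns it to the player on exit.
; While the player is inside, RotateCamera re-calls itself after a short Delay, rather than using Tick, to turn an actor toward the player.
; Both transitions briefly disable player input until just after the blend finishes.
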(event `self.Invisible Trigger.OnComponentBeginOverlap`
  (params (OverlappedComponent :type "PrimitiveComponent Object Reference") (OtherActor :type "Actor Object Reference") (OtherComp :type "PrimitiveComponent Object Reference") (OtherBodyIndex :type Integer) (bFromSweep :type Boolean) (SweepResult :type "HitResult Structure (by ref)"))
  (bind _returnvalue (`GameplayStatics.GetPlayerController` 0))
  (bind _returnvalue_2 (`GameplayStatics.GetPlayerCharacter` 0))
  (bind _asbp_player (cast `/Game/Blueprints/Player/Blueprints/BP_Player` OtherActor))
  (`PlayerController.SetViewTargetWithBlend` (`GameplayStatics.GetPlayerController` 0) null 1.0 "VTBlend_Cubic" 0.0 false)
  (set `self.Can Rotate?` true)
  (`self.RotateCamera`)
  (`self.DisableInput` _returnvalue_2 _returnvalue)
  (`KismetSystemLibrary.Delay` 1.1)
  (`self.EnableInput` _returnvalue_2 _returnvalue))

(event `self.Invisible Trigger.OnComponentEndOverlap`
  (params (OverlappedComponent :type "PrimitiveComponent Object Reference") (OtherActor :type "Actor Object Reference") (OtherComp :type "PrimitiveComponent Object Reference") (OtherBodyIndex :type Integer))
  (bind _returnvalue (`GameplayStatics.GetPlayerController` 0))
  (bind _returnvalue_2 (`GameplayStatics.GetPlayerCharacter` 0))
  (bind _asbp_player (cast `/Game/Blueprints/Player/Blueprints/BP_Player` OtherActor))
  (`PlayerController.SetViewTargetWithBlend` (`GameplayStatics.GetPlayerController` 0) _asbp_player 1.0 "VTBlend_Cubic" 0.0 false)
  (set `self.Can Rotate?` false)
  (`self.DisableInput` _returnvalue_2 _returnvalue)
  (`KismetSystemLibrary.Delay` 1.1)
  (`self.EnableInput` _returnvalue_2 _returnvalue))

(event `RotateCamera`
  (if (`self.Can Rotate?`)
    (`self.K2_SetActorRotation` "" (`KismetMathLibrary.FindLookAtRotation` (`self.K2_GetActorLocation` "") (`self.K2_GetActorLocation` (stale `self.Invisible Trigger.OnComponentBeginOverlap` _asbp_player))) false)
    (`KismetSystemLibrary.Delay` 0.005)
    (`self.RotateCamera`)))

(fn `UserConstructionScript`)