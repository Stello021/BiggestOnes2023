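; BP_CollectibleItem is an overworld pickup that adds its item to the player's inventory.
; Its PickUp event increments the Item count in BP_Player's OverworldItemsInventory map, then destroys the actor.
; Overlapping the InteractTrigger shows the interact button in the player's DialogueUI, and leaving the trigger hides it.
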(event `/Game/Blueprints/Items/BPI_PickUpItems.PickUp`
  (bind _item (`self.Item`))
  ;[1 1 1] PickUp and Collect
  (bind _asbp_player (cast `/Game/Blueprints/Player/Blueprints/BP_Player` (`GameplayStatics.GetPlayerCharacter` 0)))
  (bind _overworlditemsinventory (`/Game/Blueprints/Player/Blueprints/BP_Player.OverworldItemsInventory` _asbp_player))
  (`BlueprintMapLibrary.Map_Add` _overworlditemsinventory _item (+ (`BlueprintMapLibrary.Map_Find` _overworlditemsinventory _item) 1))
  (`self.K2_DestroyActor`))

(event `self.InteractTrigger.OnComponentBeginOverlap`
  (params (OverlappedComponent :type "PrimitiveComponent Object Reference") (OtherActor :type "Actor Object Reference") (OtherComp :type "PrimitiveComponent Object Reference") (OtherBodyIndex :type Integer) (bFromSweep :type Boolean) (SweepResult :type "HitResult Structure (by ref)"))
  ;[1 1 1] UI Interact
  (bind _asbp_player (cast `/Game/Blueprints/Player/Blueprints/BP_Player` OtherActor))
  (set `Widget.Visibility` "Visible" (`/Game/UI/Widgets/UI_Player/WB_MainUI.WB_InteractButton` (`/Game/Blueprints/Player/Blueprints/BP_Player.Dialogue UI` _asbp_player))))

(event `self.InteractTrigger.OnComponentEndOverlap`
  (params (OverlappedComponent :type "PrimitiveComponent Object Reference") (OtherActor :type "Actor Object Reference") (OtherComp :type "PrimitiveComponent Object Reference") (OtherBodyIndex :type Integer))
  ;[1 1 1] UI Interact
  (bind _asbp_player (cast `/Game/Blueprints/Player/Blueprints/BP_Player` OtherActor))
  (set `Widget.Visibility` "Hidden" (`/Game/UI/Widgets/UI_Player/WB_MainUI.WB_InteractButton` (`/Game/Blueprints/Player/Blueprints/BP_Player.Dialogue UI` _asbp_player))))

(fn `UserConstructionScript`)