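; BP_EnemyStart is an enemy spawn marker that spawns one EnemyToSpawn actor at one of its three spawn points on BeginPlay.
; It matches those points against transforms stored in the game instance to find the last one used, but the final random pick is re-rolled, so it can repeat.
; The spawned enemy receives the battle pool and arena level, and the construction script colors the arrow by PlaceEnemy.
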(event `self.ReceiveBeginPlay`
  (`self.SpawnUnit`))

(fn `SpawnUnit`
  (bind _output (`|GetArrayItem` (`self.EnemiesSpawnPoints`) (`KismetMathLibrary.RandomIntegerInRange` 0 2)))
  (bind _enemytospawn (`self.EnemyToSpawn`)
    (:`then`
      (set `self.EnemiesSpawnPoints` (`|MakeArray` (`SceneComponent.K2_GetComponentToWorld` (`self.SpawnPoint3`)) (`SceneComponent.K2_GetComponentToWorld` (`self.SpawnPoint2`)) (`SceneComponent.K2_GetComponentToWorld` (`self.SpawnPoint1`))))
      (bind _asbp_game_instance (cast `/Game/Blueprints/GameInstances/BP_GameInstance` (`GameplayStatics.GetGameInstance`)))
      (bind _output_get (set `self.As BP Game Instance` _asbp_game_instance))
      (for _array_element (`/Game/Blueprints/GameInstances/BP_GameInstance.EnemiesSpawnPoints` _output_get) :!label _label
        (for _array_element_2 (`self.EnemiesSpawnPoints`)
          (if (== _array_element_2 _array_element)
            (set `self.LastSpawnPoint` _array_element)
            (`|ExecutionSequence`
              (:`then_0`
                (break))
              (:`then_1`
                (goto _label :!via `Break`))))))
      (while (`self.NewSpawnPoint`)
        (if (not (== _output (`self.LastSpawnPoint`)))
          (set `self.NewSpawnPoint` true)))
      (bind _output_get_2 (set `self.LastSpawnPoint` _output))
      (bind _returnvalue (`|SpawnActorFromClass` _enemytospawn _output_get_2 "AdjustIfPossibleButAlwaysSpawn" "MultiplyWithRoot" null null))
      (set `/Game/Blueprints/Enemies/BP_Enemy.EnemiesPool` (`self.Enemies Pool To Battle`) _returnvalue)
      (set `/Game/Blueprints/Enemies/BP_Enemy.BattleArenaLevel` (`self.BattleArenaLevel`) _returnvalue))
    (:`else`)))

(fn `UserConstructionScript`
  (`ArrowComponent.SetArrowColor` (`self.Arrow`) (`KismetMathLibrary.SelectColor` (struct :`R` 1.0 :`A` 1.0) (struct :`R` 0.009411 :`G` 0.423918 :`B` 1.0 :`A` 1.0) (`self.PlaceEnemy`))))