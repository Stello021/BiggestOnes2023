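; Combat component for BP_UnitBase units that runs their turn-based battle actions and damage math.
; It loads level-based stats from a data table, then a Speed-derived timer requests turns from BP_BattleGameMode.
; Turns open a command widget for the player or pick a random attack or skill against the player for other units.
; Actions use AIMoveTo to approach, play a montage and return, then end or restart the turn.
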(event `self.ReceiveBeginPlay`
  (bind _asbp_unit_base (cast `/Game/Blueprints/CombatSystem/BP_UnitBase` (`self.GetOwner`)))
  (bind _output_get (set `self.UnitCharacter` _asbp_unit_base))
  (set `self.BattleTransform` (`Actor.GetTransform` _output_get)) ; Set battle transform equal to current unit transform
  (bind _returnvalue (`|GetDataTableRow` "/Game/Data/DT_BaseStatsTable.DT_BaseStatsTable" (`KismetStringLibrary.Conv_StringToName` (`KismetStringLibrary.Conv_IntToString` (`self.UnitLevel`))))
    (:`then`
      (set `self.BaseUnitStats` _returnvalue)
      (`self.BeginBattle`))))

(event `AttackCommand`
  (bind _battletransform_location (`KismetMathLibrary.BreakTransform` (`self.BattleTransform`)))
  (bind _battletransform_location_2 (`KismetMathLibrary.BreakTransform` (`self.BattleTransform`)))
  (`|AIMoveTo` (`self.UnitCharacter`) (+ (* (- (`Actor.K2_GetActorLocation` (`self.UnitTarget`)) _battletransform_location_2) 0.5) _battletransform_location_2) null 100.0
    (:`then`
      (bind _actionscommandwindow (`self.ActionsCommandWindow`)
        (:`then`
          (`Widget.RemoveFromParent` _actionscommandwindow))
        (:`else`)))
    (:`OnSuccess`
      (`|PlayMontage` (`Character.Mesh` (`self.UnitCharacter`)) (`self.AttackMontage`)
        (:`OnCompleted`
          (bind _asbp_unit_base (cast `/Game/Blueprints/CombatSystem/BP_UnitBase` (`self.GetOwner`)))
          (`/Game/Blueprints/CombatSystem/BP_UnitBase.SpendAP` _asbp_unit_base 1.0)
          (`KismetSystemLibrary.Delay` 0.0)
          (`|AIMoveTo` (`self.UnitCharacter`) _battletransform_location null
            (:`OnSuccess`
              (`AIController.K2_SetFocus` (`AIBlueprintHelperLibrary.GetAIController` (`self.UnitCharacter`)) (`self.UnitTarget`))
              (`KismetSystemLibrary.Delay` 0.75)
              (if (`self.IsTurnEnd`)
                (`self.EndUnitTurn`)
                (else
                  (`AIController.K2_ClearFocus` (`AIBlueprintHelperLibrary.GetAIController` (`self.UnitCharacter`)))
                  (`self.StartUnitTurn`))))))))))

(event `SkillCommand`
  (params (Skill :type "/Game/Blueprints/CombatSystem/Skills/BP_SkillBase Class Reference"))
  (bind _unittarget (`self.UnitTarget`))
  (bind _battletransform_location (`KismetMathLibrary.BreakTransform` (`self.BattleTransform`)))
  (bind _battletransform_location_2 (`KismetMathLibrary.BreakTransform` (`self.BattleTransform`)))
  (`|AIMoveTo` (`self.UnitCharacter`) (+ (* (- (`Actor.K2_GetActorLocation` (`self.UnitTarget`)) _battletransform_location_2) 0.5) _battletransform_location_2) null 100.0
    (:`then`
      (bind _actionscommandwindow (`self.ActionsCommandWindow`)
        (:`then`
          (`Widget.RemoveFromParent` _actionscommandwindow))
        (:`else`)))
    (:`OnSuccess`
      (bind _returnvalue (`|SpawnActorFromClass` Skill (`Actor.GetTransform` _unittarget) "Undefined" "MultiplyWithRoot" null _unittarget (`self.UnitCharacter`)))
      (`|PlayMontage` (`Character.Mesh` (`self.UnitCharacter`)) (`/Game/Blueprints/CombatSystem/Skills/BP_SkillBase.SkillMontage` _returnvalue)
        (:`OnCompleted`
          (`|AIMoveTo` (`self.UnitCharacter`) _battletransform_location null
            (:`OnSuccess`
              (`AIController.K2_SetFocus` (`AIBlueprintHelperLibrary.GetAIController` (`self.UnitCharacter`)) (`self.UnitTarget`))
              (`KismetSystemLibrary.Delay` 0.75)
              (if (`self.IsTurnEnd`)
                (`self.EndUnitTurn`)
                (else
                  (`AIController.K2_ClearFocus` (`AIBlueprintHelperLibrary.GetAIController` (`self.UnitCharacter`)))
                  (`self.StartUnitTurn`))))))))))

(fn `BeginBattle`
  (bind (_maxunitstats_hp _maxunitstats_mp _maxunitstats_attack _maxunitstats_defense _maxunitstats_elusion _maxunitstats_speed) (break `/Game/Data/ST_StatsTable` (`self.MaxUnitStats`)))
  (bind _returnvalue (`KismetSystemLibrary.K2_SetTimer` null "RequestTurn" (- 1.0 (* (`KismetMathLibrary.NormalizeToRange` (`KismetMathLibrary.FClamp` (* (`.Speed_20_1B468B424747BDD7675DF1A7E4E24C7D` (break `/Game/Data/ST_StatsModfier` (`self.UnitStatsModifier`))) (`.Speed_13_1B468B424747BDD7675DF1A7E4E24C7D` (break `/Game/Data/ST_StatsTable` (`self.BaseUnitStats`)))) 0.0 (`KismetMathLibrary.Conv_IntToDouble` _maxunitstats_speed)) 0.0 255.0) 0.01)))) ; Set timer before component's owner request turn
  (set `self.ActionTimer` _returnvalue))

(fn `CalculateBaseDamage`
  (returns (CalculatedDamage :type "Float (double-precision)"))
  (locals (NewDamage :type "Float (double-precision)" :default 0.0))
  (bind (_maxunitstats_hp _maxunitstats_mp _maxunitstats_attack) (break `/Game/Data/ST_StatsTable` (`self.MaxUnitStats`)))
  (return (`KismetMathLibrary.FClamp` (* (* (`.Attack_15_DC2FE5224229980E8E33D88671654585` (break `/Game/Data/ST_StatsTable` (`self.BaseUnitStats`))) (`.Attack_21_DC2FE5224229980E8E33D88671654585` (break `/Game/Data/ST_StatsModfier` (`self.UnitStatsModifier`)))) (`KismetMathLibrary.RandomFloatInRange` 0.9 1.1)) 0.0 (`KismetMathLibrary.Conv_IntToDouble` _maxunitstats_attack))))

(fn `CalculateDamage`
  (returns (BaseDamage :type "Float (double-precision)"))
  (bind _calculateddamage (`self.CalculateBaseDamage`))
  (return _calculateddamage))

(fn `CalculateDamageResistance`
  (params (BaseDamage :type "Float (double-precision)"))
  (returns (`New Damage` :type "Float (double-precision)"))
  (locals (Damage :type "Float (double-precision)" :default 0.0))
  (bind (_maxunitstats_hp _maxunitstats_mp _maxunitstats_attack _maxunitstats_defense) (break `/Game/Data/ST_StatsTable` (`self.MaxUnitStats`)))
  (bind _output_get (set `self.Missed` (< (`KismetMathLibrary.RandomIntegerInRange` 0 100) (* (`.Elusion_17_77C4B4FB4E51BD9A1525678D7C8A9214` (break `/Game/Data/ST_StatsTable` (`self.BaseUnitStats`))) (`.Elusion_23_77C4B4FB4E51BD9A1525678D7C8A9214` (break `/Game/Data/ST_StatsModfier` (`self.UnitStatsModifier`)))))))
  (if _output_get
    (set `local.Damage` 0.0)
    (else
      (set `local.Damage` (- BaseDamage (`KismetMathLibrary.FClamp` (* (* (`.Defense_16_E9DEBEE0409E1D16DF6395967764CB43` (break `/Game/Data/ST_StatsTable` (`self.BaseUnitStats`))) (`.Defense_22_E9DEBEE0409E1D16DF6395967764CB43` (break `/Game/Data/ST_StatsModfier` (`self.UnitStatsModifier`)))) 0.5) 0.0 (`KismetMathLibrary.Conv_IntToDouble` _maxunitstats_defense))))))
  (return (`local.Damage`)))

(fn `CalculateMagicBaseDamage`
  (params (Skill :type "/Game/Blueprints/CombatSystem/Skills/BP_SkillBase Class Reference"))
  (returns (Damage :type "Float (double-precision)"))
  (locals (FinalDamage :type "Float (double-precision)" :default 0.0))
  (return (* (* (`.Attack_15_DC2FE5224229980E8E33D88671654585` (break `/Game/Data/ST_StatsTable` (`self.BaseUnitStats`))) (`.Attack_21_DC2FE5224229980E8E33D88671654585` (break `/Game/Data/ST_StatsModfier` (`self.UnitStatsModifier`)))) (defaults `Object` (`local.Skill`)))))

(fn `EndUnitTurn`
  (bind _unitcharacter (`self.UnitCharacter`))
  (`AIController.K2_ClearFocus` (`AIBlueprintHelperLibrary.GetAIController` _unitcharacter))
  (set `self.IsTurnEnd` false)
  (set `/Game/Blueprints/CombatSystem/BP_UnitBase.CurrentAP` (`/Game/Blueprints/CombatSystem/BP_UnitBase.MaxAP` _unitcharacter) _unitcharacter)
  (`/Game/Blueprints/CombatSystem/BP_UnitBase.OnAPSpent` _unitcharacter)
  (`self.TurnEnded`)
  (`/Engine/EditorBlueprintResources/StandardMacros.IsValid` (`AIBlueprintHelperLibrary.GetAIController` (`self.UnitCharacter`))
    (:`Is Valid`
      (`self.BeginBattle`))))

(fn `RequestTurn`
  (`/Engine/EditorBlueprintResources/StandardMacros.IsValid` (`AIBlueprintHelperLibrary.GetAIController` (`self.UnitCharacter`))
    (:`Is Valid`
      (bind _asbp_battle_game_mode (cast `/Game/Blueprints/CombatSystem/BP_BattleGameMode` (`GameplayStatics.GetGameMode`)))
      (`/Game/Blueprints/CombatSystem/BP_BattleGameMode.TurnRequest` _asbp_battle_game_mode (`self.UnitCharacter`)))))

(fn `StartUnitTurn`
  (bind _unitcharacter (`self.UnitCharacter`))
  (`/Engine/EditorBlueprintResources/StandardMacros.IsValid` (`AIBlueprintHelperLibrary.GetAIController` _unitcharacter)
    (:`Is Valid`
      (if (== (`GameplayStatics.GetObjectClass` _unitcharacter) "/Game/Blueprints/CombatSystem/BP_PlayerUnit.BP_PlayerUnit_C")
        (bind _returnvalue (`|CreateWidget` "/Game/UI/Widgets/Battle/WB_ActionCommands.WB_ActionCommands_C" null (`self.UnitCharacter`) (`self.Overworld Level`)))
        (bind _output_get (set `self.ActionsCommandWindow` _returnvalue))
        (`UserWidget.AddToViewport` _output_get 0)
        (else
          (bind _returnvalue_2 (`GameplayStatics.GetActorOfClass` "/Game/Blueprints/CombatSystem/BP_PlayerUnit.BP_PlayerUnit_C"))
          (if (not (`/Game/Blueprints/CombatSystem/BP_UnitBase.isDeath` _returnvalue_2))
            (set `self.UnitTarget` _returnvalue_2)
            (switch `int` (`KismetMathLibrary.RandomIntegerInRange` 0 (`KismetArrayLibrary.Array_Length` (`self.Skills`)))
              (:`0`
                (`self.AttackCommand`))
              (:`1`
                (`self.SkillCommand` (`|GetArrayItem` (`self.Skills`))))
              (:`2`
                (`self.SkillCommand` (`|GetArrayItem` (`self.Skills`) 1)))
              (:`3`
                (`self.SkillCommand` (`|GetArrayItem` (`self.Skills`) 2))))))))
    (:`Is Not Valid`
      (`self.EndUnitTurn`))))