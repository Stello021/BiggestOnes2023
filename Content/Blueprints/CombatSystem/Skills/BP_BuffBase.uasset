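; Base Blueprint for buff skills that scale unit combat stats when spawned.
; On BeginPlay it stores its BP_UnitBase instigator and multiplies the target CombatComponent's UnitStatsModifier by UnitStatsBuff, stat by stat.
; A player instigator buffs itself, while any other instigator buffs the unit returned by GetWeakerEnemy.
; Parent BeginPlay runs afterwards, and nothing here reverts the multiplication.
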(event `self.ReceiveBeginPlay`
  (bind _returnvalue (`self.GetInstigator`))
  (bind (_hp _mp _attack _defense _accuracy _speed) (break `/Game/Data/ST_StatsModfier` (`self.Unit Stats Buff`)))
  (bind (_hp_2 _mp_2 _attack_2 _defense_2 _accuracy_2 _speed_2) (break `/Game/Data/ST_StatsModfier` (`self.Unit Stats Buff`)))
  (bind (_hp_3 _mp_3 _attack_3 _defense_3 _accuracy_3 _speed_3) (break `/Game/Data/ST_StatsModfier` (`/Game/Blueprints/CombatSystem/BP_CombatComponent.UnitStatsModifier` (`/Game/Blueprints/CombatSystem/BP_UnitBase.CombatComponent` (`self.UnitInstigator`)))))
  (bind _asbp_unit_base (cast `/Game/Blueprints/CombatSystem/BP_UnitBase` _returnvalue))
  (set `self.UnitInstigator` _asbp_unit_base)
  (if (`KismetMathLibrary.ClassIsChildOf` (`GameplayStatics.GetObjectClass` _returnvalue) "/Game/Blueprints/CombatSystem/BP_PlayerUnit.BP_PlayerUnit_C")
    (set `/Game/Blueprints/CombatSystem/BP_CombatComponent.UnitStatsModifier` (make `/Game/Data/ST_StatsModfier` (* _hp_3 _hp_2) (* _mp_3 _mp_2) (* _attack_3 _attack_2) (* _defense_3 _defense_2) (* _accuracy_3 _accuracy_2) (* _speed_3 _speed_2)) (`/Game/Blueprints/CombatSystem/BP_UnitBase.CombatComponent` (`self.UnitInstigator`)))
    (else
      (bind _weakerenemy (`self.GetWeakerEnemy`))
      (bind _combatcomponent (`/Game/Blueprints/CombatSystem/BP_UnitBase.CombatComponent` _weakerenemy))
      (bind (_hp_4 _mp_4 _attack_4 _defense_4 _accuracy_4 _speed_4) (break `/Game/Data/ST_StatsModfier` (`/Game/Blueprints/CombatSystem/BP_CombatComponent.UnitStatsModifier` _combatcomponent)))
      (set `/Game/Blueprints/CombatSystem/BP_CombatComponent.UnitStatsModifier` (make `/Game/Data/ST_StatsModfier` (* _hp_4 _hp) (* _mp_4 _mp) (* _attack_4 _attack) (* _defense_4 _defense) (* _accuracy_4 _accuracy) (* _speed_4 _speed)) _combatcomponent)))
  (`parent.ReceiveBeginPlay`))

(fn `UserConstructionScript`
  (`parent.UserConstructionScript`))