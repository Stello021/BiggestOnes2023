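; Base Blueprint for combat skill debuffs that weaken a target unit's stats.
; On BeginPlay it multiplies Attack, Defense, Accuracy and Speed in the target CombatComponent's UnitStatsModifier by UnitStatsDebuff, then calls the parent BeginPlay.
; The rebuilt modifier sets its first two fields to 1.0 instead of carrying them over.
; This graph contains no logic to revert the debuff.
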(event `self.ReceiveBeginPlay`
  (bind ((`Attack_21_DC2FE5224229980E8E33D88671654585` _attack) (`Defense_22_E9DEBEE0409E1D16DF6395967764CB43` _defense) (`Accuracy_19_77C4B4FB4E51BD9A1525678D7C8A9214` _accuracy) (`Speed_20_1B468B424747BDD7675DF1A7E4E24C7D` _speed)) (break `/Game/Data/ST_StatsModfier` (`self.Unit Stats Debuff`)))
  (bind ((`Attack_21_DC2FE5224229980E8E33D88671654585` _attack_2) (`Defense_22_E9DEBEE0409E1D16DF6395967764CB43` _defense_2) (`Accuracy_19_77C4B4FB4E51BD9A1525678D7C8A9214` _accuracy_2) (`Speed_20_1B468B424747BDD7675DF1A7E4E24C7D` _speed_2)) (break `/Game/Data/ST_StatsModfier` (`/Game/Blueprints/CombatSystem/BP_CombatComponent.UnitStatsModifier` (`/Game/Blueprints/CombatSystem/BP_UnitBase.CombatComponent` (`self.SkillTarget`)))))
  (set `/Game/Blueprints/CombatSystem/BP_CombatComponent.UnitStatsModifier` (make `/Game/Data/ST_StatsModfier` 1.0 1.0 (* _attack_2 _attack) (* _defense_2 _defense) (* _accuracy_2 _accuracy) (* _speed_2 _speed)) (`/Game/Blueprints/CombatSystem/BP_UnitBase.CombatComponent` (`self.SkillTarget`)))
  (`parent.ReceiveBeginPlay`))

(fn `UserConstructionScript`
  (`parent.UserConstructionScript`))