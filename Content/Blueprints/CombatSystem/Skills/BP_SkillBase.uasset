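; Base actor for combat skills, spawned with a unit as instigator and cleaned up when its effect ends.
; On BeginPlay it casts the instigator to BP_UnitBase and charges that unit the skill's mana and action point cost.
; The actor destroys itself when either its particle system or its Niagara component finishes.
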(event `self.ReceiveBeginPlay`
  (bind _asbp_unit_base (cast `/Game/Blueprints/CombatSystem/BP_UnitBase` (`self.GetInstigator`)))
  (`/Game/Blueprints/CombatSystem/BP_UnitBase.SpendMana` _asbp_unit_base (`KismetMathLibrary.Conv_IntToDouble` (`self.Mana`)))
  (`/Game/Blueprints/CombatSystem/BP_UnitBase.SpendAP` _asbp_unit_base (`KismetMathLibrary.Conv_IntToDouble` (`self.Cost`))))

(event `self.ParticleSystem.OnSystemFinished`
  (params (PSystem :type "ParticleSystemComponent Object Reference"))
  (`self.K2_DestroyActor` :!label _label))

(event `self.Niagara.OnSystemFinished`
  (params (PSystem :type "NiagaraComponent Object Reference"))
  (goto _label))

(fn `UserConstructionScript`)