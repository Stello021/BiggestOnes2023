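; BP_Heal is a combat skill that chooses a heal target on BeginPlay, then hands off to its parent's BeginPlay.
; A player-unit instigator targets itself.
; Any other unit instigator targets the enemy unit with the lowest CurrentHP, found by GetWeakerEnemy in the list read from BP_BattleGameMode.
; The healing itself is not implemented in these graphs.
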(event `self.ReceiveBeginPlay`
  (bind _asbp_unit_base (cast `/Game/Blueprints/CombatSystem/BP_UnitBase` (`self.GetInstigator`)))
  (if (`KismetMathLibrary.ClassIsChildOf` (`GameplayStatics.GetObjectClass` _asbp_unit_base) "/Game/Blueprints/CombatSystem/BP_PlayerUnit.BP_PlayerUnit_C")
    (set `self.SkillTarget` _asbp_unit_base)
    (else
      (bind _asbp_battle_game_mode (cast `/Game/Blueprints/CombatSystem/BP_BattleGameMode` (`GameplayStatics.GetGameMode`)))
      (set `self.Enemy Units` (`/Game/Blueprints/CombatSystem/BP_BattleGameMode.EnemyUnits` _asbp_battle_game_mode))
      (bind _weakerenemy (`self.GetWeakerEnemy`))
      (set `self.SkillTarget` _weakerenemy)))
  (`parent.ReceiveBeginPlay`))

(fn `GetWeakerEnemy`
  (returns (WeakerEnemy :type "/Game/Blueprints/CombatSystem/BP_EnemyUnitBase Object Reference"))
  (bind _enemy_units (`self.Enemy Units`))
  (bind _output (`|GetArrayItem` _enemy_units))
  (set `self.WeakerEnemy` _output)
  (`KismetArrayLibrary.Array_RemoveItem` _enemy_units _output)
  (for _array_element _enemy_units
    (if (< (`/Game/Blueprints/CombatSystem/BP_UnitBase.CurrentHP` _array_element) (`/Game/Blueprints/CombatSystem/BP_UnitBase.CurrentHP` (`self.WeakerEnemy`)))
      (set `self.WeakerEnemy` _array_element)))
  (return (`self.WeakerEnemy`)))

(fn `UserConstructionScript`
  (`parent.UserConstructionScript`))