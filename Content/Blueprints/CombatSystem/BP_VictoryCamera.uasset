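; BP_VictoryCamera is the combat system's victory camera, which records the battle result when its shot ends.
; When it becomes the view target, a timeline swings the spring arm's yaw around the scene.
; After a short delay, it saves the defeated enemy's ID and the player unit's HP and battle item inventory to the game instance.
; The node that would open the overworld map is left unconnected.
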(event `self.ReceiveBeginPlay`
  (bind _returnvalue (`GameplayStatics.GetActorOfClass` "/Game/Blueprints/CombatSystem/BP_PlayerUnit.BP_PlayerUnit_C"))
  (set `self.PlayerUnit` _returnvalue))

(event `self.K2_OnBecomeViewTarget`
  (params (PC :type "PlayerController Object Reference"))
  (bind (_direction _camerayaw) (`Timeline|CameraMovement` :!via `PlayFromStart`)
    (:`Update`
      (`SceneComponent.K2_SetRelativeRotation` (`self.SpringArm`) (`KismetMathLibrary.MakeRotator` 0.0 0.0 (+ (* _camerayaw 60.0) 30.0)) false false))
    (:`Finished`
      (`KismetSystemLibrary.Delay` 1.0)
      (bind _asbp_game_instance (cast `/Game/Blueprints/GameInstances/BP_GameInstance` (`GameplayStatics.GetGameInstance`)))
      (`KismetArrayLibrary.Array_AddUnique` (`/Game/Blueprints/GameInstances/BP_GameInstance.TutorialEnemiesKilledID` _asbp_game_instance) (`/Game/Blueprints/GameInstances/BP_GameInstance.CurrentEnemyID` _asbp_game_instance))
      (set `/Game/Blueprints/GameInstances/BP_GameInstance.PlayerCurrentHP` (`/Game/Blueprints/CombatSystem/BP_UnitBase.CurrentHP` (`self.PlayerUnit`)) _asbp_game_instance)
      (set `/Game/Blueprints/GameInstances/BP_GameInstance.PlayerCurrentInventory` (`/Game/Blueprints/CombatSystem/BP_PlayerUnit.BattleItemsInventory` (`self.PlayerUnit`)) _asbp_game_instance))))

(fn `UserConstructionScript`)