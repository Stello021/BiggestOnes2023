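; Game mode for turn-based battles that switches the view to the battle camera, tracks player and enemy units, and sequences their turns.
; Units request turns into a duplicate-free queue, and a DoOnce gate lets only one start at a time.
; The front unit's CombatComponent starts the turn and gets a turn-ended binding, while units without an AI controller are skipped.
; ReadyNextTurn reopens the gate, and RemoveUnitFromBattle clears units from the tracked references.
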(event `self.ReceiveBeginPlay`
  (bind _returnvalue (`GameplayStatics.GetActorOfClass` "/Game/Blueprints/CombatSystem/BP_BattleCamera.BP_BattleCamera_C"))
  (set `self.MainBattleCamera` _returnvalue)
  (`PlayerController.SetViewTargetWithBlend` (`GameplayStatics.GetPlayerController` 0) (`self.MainBattleCamera`) 0.0 "VTBlend_Linear" 0.0 false)
  (bind _returnvalue_2 (`GameplayStatics.GetActorOfClass` "/Game/Blueprints/CombatSystem/BP_PlayerUnit.BP_PlayerUnit_C"))
  (set `self.PlayerUnit` _returnvalue_2)
  (bind _outactors (`GameplayStatics.GetAllActorsOfClass` "/Game/Blueprints/CombatSystem/BP_EnemyUnitBase.BP_EnemyUnitBase_C"))
  (set `self.EnemyUnits` _outactors))

(event `TurnRequest`
  (params (Unit :type "/Game/Blueprints/CombatSystem/BP_UnitBase Object Reference"))
  (`KismetArrayLibrary.Array_AddUnique` (`self.TurnOrder`) Unit) ; Add Unique to prevent duplicates of the same unit inside list, if the unit is already present don't readd, otherwise add it
  (`self.StartTurn`))

(event `StartTurn`
  (bind _output (`|GetArrayItem` (`self.TurnOrder`)))
  (bind _combatcomponent (`/Game/Blueprints/CombatSystem/BP_UnitBase.CombatComponent` _output))
  (`/Engine/EditorBlueprintResources/StandardMacros.DoOnce` false :!label _label ; Avoid that two or more characters start their turns at the same time
    (:`Completed`
      (if (`KismetArrayLibrary.Array_IsValidIndex` (`self.TurnOrder`))
        (`/Engine/EditorBlueprintResources/StandardMacros.IsValid` (`AIBlueprintHelperLibrary.GetAIController` _output)
          (:`Is Valid`
            (`/Game/Blueprints/CombatSystem/BP_CombatComponent.StartUnitTurn` _combatcomponent)
            (add `/Game/Blueprints/CombatSystem/BP_CombatComponent.TurnEnded` _combatcomponent (`|CreateDelegate` :!event `ReadyNextTurn`)) ; Call the event linked to Combat component EventDispatcher Turn Ended specific for the single unit
            (`KismetArrayLibrary.Array_Remove` (`self.TurnOrder`)) ; Remove unit from the array when its turn ended
          )
          (:`Is Not Valid`
            (`KismetArrayLibrary.Array_Remove` (`self.TurnOrder`)) ; Remove unit from the array when its turn ended
            (`self.ReadyNextTurn`)))
        (else
          (`self.ReadyNextTurn`) ; if unit is not valid pass to the next
        )))))

(event `ReadyNextTurn`
  (`|ExecutionSequence`
    (:`then_0`
      (goto _label :!via `Reset`))
    (:`then_1`
      (if (`KismetArrayLibrary.Array_IsValidIndex` (`self.TurnOrder`))
        (`self.StartTurn`)))))

(fn `RemoveUnitFromBattle`
  (params (Unit :type "/Game/Blueprints/CombatSystem/BP_UnitBase Object Reference"))
  (bind _asbp_enemy_unit_base (cast `/Game/Blueprints/CombatSystem/BP_EnemyUnitBase` Unit)
    (:`then`
      (`KismetArrayLibrary.Array_RemoveItem` (`self.EnemyUnits`) _asbp_enemy_unit_base))
    (:`CastFailed`
      (set `self.PlayerUnit` null))))

(fn `UserConstructionScript`)