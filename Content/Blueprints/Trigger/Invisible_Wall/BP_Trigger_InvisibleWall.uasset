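; Invisible wall trigger that shows a text message while the player overlaps it and can remove another linked wall.
; On player overlap it creates a WB_WallMessagge widget with its TextLine, then passes NextObjToDestroy (box or sphere wall) to DestroySelectedActor.
; End overlap removes the widget.
; On BeginPlay it destroys itself if its display name is in the GameInstance's ActorToDestroy list, so removals can carry over.
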(event `self.ReceiveBeginPlay`
  (bind _asbp_game_instance (cast `/Game/Blueprints/GameInstances/BP_GameInstance` (`GameplayStatics.GetGameInstance`)))
  (if (!= (`KismetArrayLibrary.Array_Find` (`/Game/Blueprints/GameInstances/BP_GameInstance.ActorToDestroy` _asbp_game_instance) (`KismetSystemLibrary.GetDisplayName` self)) -1)
    (`self.K2_DestroyActor`)))

(event `self.Invisible Trigger.OnComponentBeginOverlap`
  (params (OverlappedComponent :type "PrimitiveComponent Object Reference") (OtherActor :type "Actor Object Reference") (OtherComp :type "PrimitiveComponent Object Reference") (OtherBodyIndex :type Integer) (bFromSweep :type Boolean) (SweepResult :type "HitResult Structure (by ref)"))
  (bind _next_obj_todestroy (`self.Next_Obj_ToDestroy`))
  (cast `/Game/Blueprints/Player/Blueprints/BP_Player` OtherActor)
  (bind _returnvalue (`|CreateWidget` "/Game/UI/Widgets/WallCollision/WB_WallMessagge.WB_WallMessagge_C"))
  (bind _output_get (set `self.Widget_Wall` _returnvalue))
  (`UserWidget.AddToViewport` _output_get 0)
  (set `TextBlock.Text` (`self.TextLine`) (`/Game/UI/Widgets/WallCollision/WB_WallMessagge.TB_TextLine` _output_get))
  (`/Engine/EditorBlueprintResources/StandardMacros.IsValid` _next_obj_todestroy
    (:`Is Valid`
      (bind _asbp_trigger_invisible_wall (cast `/Game/Blueprints/Trigger/Invisible_Wall/BP_Trigger_InvisibleWall` _next_obj_todestroy)
        (:`then`
          (`self.DestroySelectedActor` _asbp_trigger_invisible_wall))
        (:`CastFailed`
          (bind _asbp_trigger_invisible_wall_sphere (cast `/Game/Blueprints/Trigger/Invisible_Wall/BP_Trigger_InvisibleWallSphere` _next_obj_todestroy))
          (`self.DestroySelectedActor` _asbp_trigger_invisible_wall_sphere))))))

(event `self.Invisible Trigger.OnComponentEndOverlap`
  (params (OverlappedComponent :type "PrimitiveComponent Object Reference") (OtherActor :type "Actor Object Reference") (OtherComp :type "PrimitiveComponent Object Reference") (OtherBodyIndex :type Integer))
  (bind _widget_wall (`self.Widget_Wall`))
  (`/Engine/EditorBlueprintResources/StandardMacros.IsValid` _widget_wall
    (:`Is Valid`
      (`Widget.RemoveFromParent` _widget_wall))))

(fn `UserConstructionScript`
  (`parent.UserConstructionScript`))