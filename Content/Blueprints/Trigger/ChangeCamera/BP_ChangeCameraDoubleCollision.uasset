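; Trigger actor that switches the player's view to a placed camera while the player is in its area, using two separate collision volumes.
; When BP_Player begins overlapping EnterCollision, player controller 0 blends its view target to the actor spawned by the Camera child actor component.
; When BP_Player stops overlapping ExitCollision, the view blends back to the player, with both transitions sharing the BlendTime variable.
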(event `self.EnterCollision.OnComponentBeginOverlap`
  (params (OverlappedComponent :type "PrimitiveComponent Object Reference") (OtherActor :type "Actor Object Reference") (OtherComp :type "PrimitiveComponent Object Reference") (OtherBodyIndex :type Integer) (bFromSweep :type Boolean) (SweepResult :type "HitResult Structure (by ref)"))
  (cast `/Game/Blueprints/Player/Blueprints/BP_Player` OtherActor)
  (`PlayerController.SetViewTargetWithBlend` (`GameplayStatics.GetPlayerController` 0) (`ChildActorComponent.ChildActor` (`self.Camera`)) (`self.Blend Time`) "VTBlend_Linear" 0.0 false))

(event `self.ExitCollision.OnComponentEndOverlap`
  (params (OverlappedComponent :type "PrimitiveComponent Object Reference") (OtherActor :type "Actor Object Reference") (OtherComp :type "PrimitiveComponent Object Reference") (OtherBodyIndex :type Integer))
  (bind _asbp_player (cast `/Game/Blueprints/Player/Blueprints/BP_Player` OtherActor))
  (`PlayerController.SetViewTargetWithBlend` (`GameplayStatics.GetPlayerController` 0) _asbp_player (`self.Blend Time`) "VTBlend_Linear" 0.0 false))

(fn `UserConstructionScript`
  (`parent.UserConstructionScript`))