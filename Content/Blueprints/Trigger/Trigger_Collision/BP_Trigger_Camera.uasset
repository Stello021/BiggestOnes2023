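; BP_Trigger_Camera is a trigger volume that switches the player's view to a placed child-actor camera while BP_Player stands inside it.
; Overlap begin and end blend the view target to that camera and back to the player over one second.
; Player input is disabled briefly during each blend.
; While the camera is active, Tick rotates it to keep looking at the player character.
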(event `self.Invisible Trigger.OnComponentBeginOverlap`
  (params (OverlappedComponent :type "PrimitiveComponent Object Reference") (OtherActor :type "Actor Object Reference") (OtherComp :type "PrimitiveComponent Object Reference") (OtherBodyIndex :type Integer) (bFromSweep :type Boolean) (SweepResult :type "HitResult Structure (by ref)"))
  (cast `/Game/Blueprints/Player/Blueprints/BP_Player` OtherActor)
  (`PlayerController.SetViewTargetWithBlend` (`GameplayStatics.GetPlayerController` 0) (`ChildActorComponent.ChildActor` (`self.Camera`)) 1.0 "VTBlend_Linear" 0.0 false)
  (set `self.IsMainCamera` true)
  (`self.DisableInput` (`GameplayStatics.GetPlayerCharacter` 0) (`GameplayStatics.GetPlayerController` 0))
  (`KismetSystemLibrary.Delay` 1.1)
  (`self.EnableInput` (`GameplayStatics.GetPlayerCharacter` 0) (`GameplayStatics.GetPlayerController` 0)))

(event `self.Invisible Trigger.OnComponentEndOverlap`
  (params (OverlappedComponent :type "PrimitiveComponent Object Reference") (OtherActor :type "Actor Object Reference") (OtherComp :type "PrimitiveComponent Object Reference") (OtherBodyIndex :type Integer))
  (bind _asbp_player (cast `/Game/Blueprints/Player/Blueprints/BP_Player` OtherActor))
  (`PlayerController.SetViewTargetWithBlend` (`GameplayStatics.GetPlayerController` 0) _asbp_player 1.0 "VTBlend_Linear" 0.0 false)
  (set `self.IsMainCamera` false)
  (`self.DisableInput` (`GameplayStatics.GetPlayerCharacter` 0) (`GameplayStatics.GetPlayerController` 0))
  (`KismetSystemLibrary.Delay` 1.1)
  (`self.EnableInput` (`GameplayStatics.GetPlayerCharacter` 0) (`GameplayStatics.GetPlayerController` 0)))

(event `self.ReceiveTick`
  (params (DeltaSeconds :type "Float (single-precision)"))
  (bind _childactor (`ChildActorComponent.ChildActor` (`self.Camera`)))
  (if (`self.IsMainCamera`)
    (`self.K2_SetActorRotation` _childactor (`KismetMathLibrary.FindLookAtRotation` (`self.K2_GetActorLocation` _childactor) (`self.K2_GetActorLocation` (`GameplayStatics.GetPlayerCharacter` 0))) false)))

(fn `UserConstructionScript`
  (`parent.UserConstructionScript`))