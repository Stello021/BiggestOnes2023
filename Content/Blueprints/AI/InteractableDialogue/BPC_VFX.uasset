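; BPC_VFX is an interactable Blueprint that removes its PLocate component once the player has used it.
; Player overlap arms removal with no end-overlap reset; Tick then polls for E release to destroy the component.
; The component's display name, not the actor's, is stored in the GameInstance's VFXActive list, which BeginPlay checks to destroy it again on later loads.
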(event `self.ReceiveBeginPlay`
  (`parent.ReceiveBeginPlay`)
  (bind _asbp_game_instance (cast `/Game/Blueprints/GameInstances/BP_GameInstance` (`GameplayStatics.GetGameInstance`)))
  (if (!= (`KismetArrayLibrary.Array_Find` (`/Game/Blueprints/GameInstances/BP_GameInstance.VFX_Active` _asbp_game_instance) (`KismetSystemLibrary.GetDisplayName` (`self.P_Locate`))) -1)
    (`ActorComponent.K2_DestroyComponent` (`self.P_Locate`))))

(event `self.ReceiveActorBeginOverlap`
  (params (OtherActor :type "Actor Object Reference"))
  (cast `/Game/Blueprints/Player/Blueprints/BP_Player` OtherActor)
  (set `self.canDestroy` true))

(event `self.ReceiveTick`
  (params (DeltaSeconds :type "Float (single-precision)"))
  (`/Engine/EditorBlueprintResources/StandardMacros.IsValid` (`self.P_Locate`)
    (:`Is Valid`
      (if (and (`PlayerController.WasInputKeyJustReleased` (`GameplayStatics.GetPlayerController` 0) "E") (`self.canDestroy`))
        (set `self.canDestroy` false)
        (`ActorComponent.K2_DestroyComponent` (`self.P_Locate`))
        (bind _asbp_game_instance (cast `/Game/Blueprints/GameInstances/BP_GameInstance` (`GameplayStatics.GetGameInstance`)))
        (`KismetArrayLibrary.Array_Add` (`/Game/Blueprints/GameInstances/BP_GameInstance.VFX_Active` _asbp_game_instance) (`KismetSystemLibrary.GetDisplayName` (`self.P_Locate`)))
        (`KismetSystemLibrary.PrintString` "Added")))))

(fn `UserConstructionScript`
  (`parent.UserConstructionScript`))