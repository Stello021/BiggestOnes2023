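; Trigger Blueprint that makes a Wilp appear or disappear when the player overlaps its TriggerSpawn volume.
; The Wilp starts at zero scale on BeginPlay.
; Each player overlap shows SpawnAura, waits briefly, then flips IsVisible to play either a grow or shrink timeline on the Wilp's scale.
; Both timelines share a delay that hides the aura shortly after scaling begins.
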(event `self.ReceiveBeginPlay`
  (`parent.ReceiveBeginPlay`)
  (`SceneComponent.SetRelativeScale3D` (`self.Wilp`) (0.0 0.0 0.0)))

(event `self.ReceiveTick`
  (params (DeltaSeconds :type "Float (single-precision)"))
  (`parent.ReceiveTick` DeltaSeconds))

(event `self.Trigger Spawn.OnComponentBeginOverlap`
  (params (OverlappedComponent :type "PrimitiveComponent Object Reference") (OtherActor :type "Actor Object Reference") (OtherComp :type "PrimitiveComponent Object Reference") (OtherBodyIndex :type Integer) (bFromSweep :type Boolean) (SweepResult :type "HitResult Structure (by ref)"))
  (bind _wilp (`self.Wilp`))
  (cast `/Game/Blueprints/Player/Blueprints/BP_Player` OtherActor)
  (`SceneComponent.SetVisibility` (`self.SpawnAura`) true false)
  (`KismetSystemLibrary.Delay` 1.0)
  (bind _output_get (set `self.IsVisible` (not (`self.IsVisible`))))
  (if _output_get
    (bind (_direction _scale_to_1) (`Timeline|Scale 0 To 1` :!via `PlayFromStart`)
      (:`Update`
        (`SceneComponent.SetRelativeScale3D` _wilp (`KismetMathLibrary.MakeVector` _scale_to_1 _scale_to_1 _scale_to_1))))
    (else
      (bind (_direction_2 _newtrack_0) (`Timeline|Scale 1 To 0` :!via `PlayFromStart`)
        (:`Update`
          (`SceneComponent.SetRelativeScale3D` _wilp (`KismetMathLibrary.MakeVector` _newtrack_0 _newtrack_0 _newtrack_0))))))
  (`KismetSystemLibrary.Delay` 1.0)
  (`SceneComponent.SetVisibility` (`self.SpawnAura`) false false))

(fn `UserConstructionScript`
  (`parent.UserConstructionScript`))