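; First tree AI actor that opens the Tutorial_Castle intro with a cutscene and starts a dialogue behavior tree.
; BeginPlay records its name in the game instance, destroying itself if already listed, and plays the sequence with pawn input disabled if unseen.
; Tick polls Interact and SkipAnimation key mappings while FirstTime holds.
; Skipping ends the cutscene and shows tutorial commands; interacting removes that widget and runs DialogueTree once.
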(event `self.ReceiveBeginPlay`
  (bind _returnvalue (`KismetSystemLibrary.GetObjectName` self))
  (`parent.ReceiveBeginPlay`)
  (bind _asbp_game_instance (cast `/Game/Blueprints/GameInstances/BP_GameInstance` (`GameplayStatics.GetGameInstance`)))
  (bind _actortodestroy (`/Game/Blueprints/GameInstances/BP_GameInstance.ActorToDestroy` _asbp_game_instance))
  (if (== (`KismetArrayLibrary.Array_Find` _actortodestroy _returnvalue) -1)
    (`KismetArrayLibrary.Array_AddUnique` _actortodestroy _returnvalue)
    (bind _returnvalue_2 (`GameplayStatics.GetCurrentLevelName` true))
    (if (`KismetStringLibrary.EqualEqual_StrStr` _returnvalue_2 "Tutorial_Castle")
      (if (not (`/Game/Blueprints/GameInstances/BP_GameInstance.IsPlayedCutScene` _asbp_game_instance))
        (`self.DisableInput` (`GameplayStatics.GetPlayerPawn` 0) (`GameplayStatics.GetPlayerController` 0))
        (bind (_outactor _returnvalue_3) (`LevelSequencePlayer.CreateLevelSequencePlayer` (`self.Level Sequence`)))
        (bind _output_get (set `self.CutScene` _returnvalue_3))
        (`MovieSceneSequencePlayer.Play` _output_get)))
    (else
      (`self.K2_DestroyActor`))))

(event `self.ReceiveTick`
  (params (DeltaSeconds :type "Float (single-precision)"))
  (bind _cutscene (`self.CutScene`))
  (if (`self.FirstTime`)
    (if (`self.Input Skip`)
      (if (`MovieSceneSequencePlayer.IsPlaying` _cutscene)
        (`MovieSceneSequencePlayer.GoToEndAndStop` _cutscene)
        (bind _returnvalue (`|CreateWidget` "/Game/UI/Widgets/UI_Player/WB_TutorialComands.WB_TutorialComands_C" (`GameplayStatics.GetPlayerController` 0)))
        (`UserWidget.AddToViewport` _returnvalue 0))
      (elif (`self.Input Interaction`)
        (`Widget.RemoveFromParent` _returnvalue)
        (`AIController.RunBehaviorTree` (`AIBlueprintHelperLibrary.GetAIController` self) (`self.Dialogue Tree`))
        (set `self.FirstTime` false)))))

(fn `Input Interaction`
  (returns (KeyPressed :type Boolean))
  (locals (KeyPressedd :type Boolean))
  (if (`PlayerController.WasInputKeyJustPressed` (`GameplayStatics.GetPlayerController` 0) "AnyKey")
    (for _array_element (`InputSettings.GetActionMappingByName` (`InputSettings.GetInputSettings`) "Interact")
      (set `local.KeyPressedd` (`PlayerController.WasInputKeyJustPressed` (`GameplayStatics.GetPlayerController` 0) (`.Key` (break `InputActionKeyMapping` _array_element)))))
    (return (`local.KeyPressedd`))))

(fn `Input Skip`
  (returns (KeyPressed :type Boolean))
  (locals (NewLocalVar :type Boolean))
  (if (`PlayerController.WasInputKeyJustPressed` (`GameplayStatics.GetPlayerController` 0) "AnyKey")
    (for _array_element (`InputSettings.GetActionMappingByName` (`InputSettings.GetInputSettings`) "SkipAnimation")
      (set `local.NewLocalVar` (`PlayerController.WasInputKeyJustPressed` (`GameplayStatics.GetPlayerController` 0) (`.Key` (break `InputActionKeyMapping` _array_element)))))
    (return (`local.NewLocalVar`))))

(fn `UserConstructionScript`
  (`parent.UserConstructionScript`))