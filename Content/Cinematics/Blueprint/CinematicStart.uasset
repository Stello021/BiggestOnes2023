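; CinematicStart is a trigger actor that plays the GoBack level sequence when the player character enters its Box.
; BeginPlay creates the sequence player, and the overlap event disables player input and starts playback.
; A one-shot timer set to the sequence's duration re-enables input, rather than a binding to the player's finished event.
; The trigger has no once-only guard, so each new overlap replays the cutscene.
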(event `self.ReceiveBeginPlay`
  (bind (_outactor _returnvalue) (`LevelSequencePlayer.CreateLevelSequencePlayer` "/Game/Cinematics/Sequences/GoBack.GoBack"))
  (set `self.Cutscene` _returnvalue))

(event `self.Box.OnComponentBeginOverlap`
  (params (OverlappedComponent :type "PrimitiveComponent Object Reference") (OtherActor :type "Actor Object Reference") (OtherComp :type "PrimitiveComponent Object Reference") (OtherBodyIndex :type Integer) (bFromSweep :type Boolean) (SweepResult :type "HitResult Structure (by ref)"))
  (bind _returnvalue (`GameplayStatics.GetPlayerCharacter` 0))
  (bind _cutscene (`self.Cutscene`))
  (if (== OtherActor _returnvalue)
    (`self.DisableInput` _returnvalue (`GameplayStatics.GetPlayerController` 0))
    (`MovieSceneSequencePlayer.Play` _cutscene)
    (`KismetSystemLibrary.K2_SetTimerDelegate` (delegate `EnableMovment`) (`TimeManagementBlueprintLibrary.Conv_QualifiedFrameTimeToSeconds` (`MovieSceneSequencePlayer.GetDuration` _cutscene)))))

(event `EnableMovment`
  (`self.EnableInput` (`GameplayStatics.GetPlayerCharacter` 0) (`GameplayStatics.GetPlayerController` 0)))

(fn `UserConstructionScript`)