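; Interactive treasure chest that the player opens and closes with E while inside its box trigger.
; Overlap toggles input, a gate and the prompt widget, and shows the coins if ThereIsGold is set.
; Separate open and close timelines animate the lid and chest body from cached initial transforms, with BlockAnim ignoring presses mid-animation.
; Opening a chest with gold spawns a one-shot effect and lights a point light, which closing hides.
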(event `self.ReceiveBeginPlay`
  (bind _meshchest (`self.MeshChest`))
  ;[1 1 1] Variables
  (set `self.chest_open` false)
  (set `self.init_rot` (`SceneComponent.K2_GetComponentRotation` (`self.lid`)))
  (set `self.block_anim` false)
  (set `self.initChest_loc` (`SceneComponent.K2_GetComponentLocation` _meshchest))
  (set `self.initChest_rot` (`SceneComponent.K2_GetComponentRotation` _meshchest)))

(event `Key|E`
  (params (Key :type "Key Structure"))
  (bind _pointlight (`self.PointLight`))
  (bind (_initchest_loc_x _initchest_loc_y _initchest_loc_z) (`KismetMathLibrary.BreakVector` (`self.initChest_loc`)))
  (bind (_initchest_rot_roll _initchest_rot_pitch _initchest_rot_yaw) (`KismetMathLibrary.BreakRotator` (`self.initChest_rot`)))
  (bind (_initchest_rot_roll_2 _initchest_rot_pitch_2 _initchest_rot_yaw_2) (`KismetMathLibrary.BreakRotator` (`self.initChest_rot`)))
  (bind (_init_rot_roll _init_rot_pitch _init_rot_yaw) (`KismetMathLibrary.BreakRotator` (`self.init_rot`)))
  (bind _meshchest (`self.MeshChest`))
  (bind (_init_rot_roll_2 _init_rot_pitch_2 _init_rot_yaw_2) (`KismetMathLibrary.BreakRotator` (`self.init_rot`)))
  (:`Pressed`
    (if (not (`self.block_anim`))
      (`/Engine/EditorBlueprintResources/StandardMacros.Gate` true :!label _label
        (:`Exit`
          (set `self.block_anim` true)
          (if (`self.chest_open`)
            ;[1 1 1] Close Chest Animation
            (bind (_direction _anim_chest_close _anim_chest_up _anim_allchestrot) (`Timeline|Timeline_1` :!via `PlayFromStart`)
              (:`Update`
                (`SceneComponent.K2_SetWorldRotation` (`self.lid`) (`KismetMathLibrary.MakeRotator` _init_rot_roll_2 (+ _anim_chest_close _init_rot_pitch_2) _init_rot_yaw_2) false false)
                (`SceneComponent.K2_SetWorldLocation` _meshchest (`KismetMathLibrary.MakeVector` _initchest_loc_x _initchest_loc_y (+ _anim_chest_up _initchest_loc_z)) false false)
                (`SceneComponent.K2_SetWorldRotation` _meshchest (`KismetMathLibrary.MakeRotator` (+ _anim_allchestrot _initchest_rot_roll) _initchest_rot_pitch _initchest_rot_yaw) false false))
              (:`Finished`
                (`SceneComponent.SetVisibility` _pointlight false false)
                (set `self.chest_open` false)
                (set `self.block_anim` false :!label _label_2)
                (`SceneComponent.SetVisibility` (`self.Widget`) (and (`self.isOverlap`) (== (`self.chest_open`) false)) false)
                (set `self.once` false)))
            (else
              ;[1 1 1] Open Chest Animation
              (`SceneComponent.SetVisibility` (`self.Widget`) false false)
              (bind (_direction_2 _anim_open_chest _anim_chestdown) (`Timeline|Timeline_0` :!via `PlayFromStart`)
                (:`Update`
                  (`SceneComponent.K2_SetWorldRotation` (`self.lid`) (`KismetMathLibrary.MakeRotator` _init_rot_roll (+ _anim_open_chest _init_rot_pitch) _init_rot_yaw) false false)
                  (`SceneComponent.K2_SetWorldRotation` (`self.MeshChest`) (`KismetMathLibrary.MakeRotator` _initchest_rot_roll_2 (+ _anim_chestdown _initchest_rot_pitch_2) _initchest_rot_yaw_2) false false)
                  (if (`self.ThereIsGold`)
                    (if (!= (`self.once`) true)
                      (set `self.once` true)
                      (`NiagaraFunctionLibrary.SpawnSystemAtLocation` "/Game/Asset/StylizedRuins/FX/P_ChestOpenEffect.P_ChestOpenEffect" (`self.K2_GetActorLocation`))
                      (`SceneComponent.SetVisibility` _pointlight true false))))
                (:`Finished`
                  (set `self.chest_open` true)
                  (goto _label_2))))))))))

(event `self.Box.OnComponentBeginOverlap`
  (params (OverlappedComponent :type "PrimitiveComponent Object Reference") (OtherActor :type "Actor Object Reference") (OtherComp :type "PrimitiveComponent Object Reference") (OtherBodyIndex :type Integer) (bFromSweep :type Boolean) (SweepResult :type "HitResult Structure (by ref)"))
  (set `self.isOverlap` true)
  (`SceneComponent.SetVisibility` (`self.Widget`) (!= (`self.chest_open`) true) false)
  (`SceneComponent.SetVisibility` (`self.Coins`) (`self.ThereIsGold`) false)
  (`self.EnableInput` (`GameplayStatics.GetPlayerController` 0))
  (goto _label :!via `Open`))

(event `self.Box.OnComponentEndOverlap`
  (params (OverlappedComponent :type "PrimitiveComponent Object Reference") (OtherActor :type "Actor Object Reference") (OtherComp :type "PrimitiveComponent Object Reference") (OtherBodyIndex :type Integer))
  (set `self.isOverlap` false)
  (`SceneComponent.SetVisibility` (`self.Widget`) false false)
  (`self.DisableInput` null)
  (goto _label :!via `Close`))

(fn `UserConstructionScript`)