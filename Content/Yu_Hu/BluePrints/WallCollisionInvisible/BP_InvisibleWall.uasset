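; BP_InvisibleWall is an overlap actor that shows a text message to the player and removes a linked wall.
; When BP_Player enters, it creates a WB_WallMessagge widget showing TextLine, then removes the widget on end overlap.
; Entering also destroys WallToDestroy if valid, whose OnDestroyed event sets a flag that skips further destroy attempts.
; Nodes for disabling and re-enabling player input are present but never run.
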(event `self.ReceiveActorBeginOverlap`
  (params (OtherActor :type "Actor Object Reference"))
  (bind _wall_to_destroy (`self.Wall To Destroy`))
  (cast `/Game/Blueprints/Player/Blueprints/BP_Player` OtherActor)
  (bind _returnvalue (`|CreateWidget` "/Game/UI/Widgets/WallCollision/WB_WallMessagge.WB_WallMessagge_C"))
  (`UserWidget.AddToViewport` _returnvalue 0)
  (set `TextBlock.Text` (`self.TextLine`) (`/Game/UI/Widgets/WallCollision/WB_WallMessagge.TB_TextLine` _returnvalue))
  (if (not (`self.Wall Is Destroyed`))
    (`/Engine/EditorBlueprintResources/StandardMacros.IsValid` _wall_to_destroy
      (:`Is Valid`
        (`self.K2_DestroyActor` _wall_to_destroy)))))

(event `self.ReceiveActorEndOverlap`
  (params (OtherActor :type "Actor Object Reference"))
  (`Widget.RemoveFromParent` (stale `self.ReceiveActorBeginOverlap` _returnvalue)))

(event `self.Wall To Destroy.OnDestroyed`
  (params (DestroyedActor :type "Actor Object Reference"))
  (set `self.Wall Is Destroyed` true))

(fn `UserConstructionScript`)