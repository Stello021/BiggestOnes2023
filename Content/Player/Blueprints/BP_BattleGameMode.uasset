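; Battle game mode that runs a turn queue for player and enemy units, one active turn at a time.
; TurnRequest adds units to TurnOrder without duplicates, then tries StartTurn, which a DoOnce gates against simultaneous turns.
; StartTurn starts the first unit's turn through its CombatComponent, binds to that component's TurnEnded dispatcher and removes the unit from the queue.
; ReadyNextTurn resets the gate and starts the next queued turn.
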(event `TurnRequest`
  (params (Unit :type "/Game/Blueprints/CombatSystem/BP_UnitBase Object Reference"))
  (`KismetArrayLibrary.Array_AddUnique` (`self.TurnOrder`)) ; Add Unique to prevent duplicates of the same unit inside list, if the unit is already present don't readd, otherwise add it
  (`self.StartTurn`))

(event `StartTurn`
  (bind _combatcomponent (`/Game/Blueprints/CombatSystem/BP_UnitBase.CombatComponent` (`|GetArrayItem` (`self.TurnOrder`))))
  (`/Engine/EditorBlueprintResources/StandardMacros.DoOnce` false :!label _label ; Avoid that two or more characters start their turns at the same time
    (:`Completed`
      (if (`KismetArrayLibrary.Array_IsValidIndex` (`self.TurnOrder`))
        (`/Game/Blueprints/CombatSystem/BP_CombatComponent.StartUnitTurn` _combatcomponent)
        (add `/Game/Blueprints/CombatSystem/BP_CombatComponent.TurnEnded` _combatcomponent (`|CreateDelegate` :!event `ReadyNextTurn`)) ; Call the event linked to Combat component EventDispatcher Turn Ended specific for the single unit
        (`KismetArrayLibrary.Array_Remove` (`self.TurnOrder`)) ; Remove unit from the array when its turn ended
        (else
          (`self.ReadyNextTurn`) ; if unit is not valid pass to the next
        )))))

(event `ReadyNextTurn`
  (`|ExecutionSequence`
    (:`then_0`
      (goto _label :!via `Reset`))
    (:`then_1`
      (if (`KismetArrayLibrary.Array_IsValidIndex` (`self.TurnOrder`))
        (`self.StartTurn`)))))

(fn `UserConstructionScript`)