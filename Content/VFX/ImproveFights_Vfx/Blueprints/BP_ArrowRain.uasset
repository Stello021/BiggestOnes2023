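; BP_ArrowRain is a VFX spawner actor that fires repeating volleys of Arrow actors.
; After a start delay on BeginPlay, the self-calling NextArrow event spawns arrows at short random intervals until its counter reaches ArrowCount.
; Each arrow gets a random world-space offset from the actor and a random direction within a narrow cone around its forward vector.
; After a long fixed pause, the counter resets and the next volley starts, looping indefinitely.
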(event `NextArrow`
  (`|SpawnActorFromClass` (`self.Arrow`) (`KismetMathLibrary.MakeTransform` (+ (`self.K2_GetActorLocation`) (`KismetMathLibrary.MakeVector` (`KismetMathLibrary.RandomFloatInRange` -100.0 100.0) (`KismetMathLibrary.RandomFloatInRange` -10.0 100.0) (`KismetMathLibrary.RandomFloatInRange` -50.0 50.0))) (`KismetMathLibrary.MakeRotFromX` (`KismetMathLibrary.RandomUnitVectorInConeInDegrees` (`self.GetActorForwardVector`) 10.0))) "Undefined" "SelectDefaultAtRuntime" null null :!label _label)
  (`KismetSystemLibrary.Delay` (`KismetMathLibrary.RandomFloatInRange` 0.1 0.3))
  (if (< (`self.Arrows`) (`self.Arrow_Count`))
    (`/Engine/EditorBlueprintResources/StandardMacros.IncrementFloat` (`self.Arrows`)
      (:`  `
        (`self.NextArrow`)))
    (else
      (`KismetSystemLibrary.Delay` 14.5)
      (set `self.Arrows` 1.0)
      (`self.NextArrow`))))

(event `self.ReceiveBeginPlay`
  (`KismetSystemLibrary.Delay` (`self.Start_Delay`))
  (goto _label))

(fn `UserConstructionScript`)