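; Actor Blueprint that repeatedly spawns stylized VR explosion Niagara or particle effects at its own location, apparently for showcasing the effect pack.
; Variant picks the Energy or Effect family and Level picks one of three systems in it.
; BeginPlay staggers the first burst by a delay derived from Level and Variant, then the Again event re-calls itself to repeat every six seconds.
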(event `Again`
  (bind _returnvalue (`self.K2_GetActorLocation`))
  (bind _returnvalue_2 (`self.K2_GetActorLocation`))
  (`KismetSystemLibrary.Delay` 6.0)
  (if (== (`self.Variant`) 1) :!label _label
    (switch `int` (`self.Level`)
      (:`1`
        (`NiagaraFunctionLibrary.SpawnSystemAtLocation` "/Game/VFX/Stylized_VFX_StPack/VR/VR_Particles/P_VR_ExplosionEnergy_01.P_VR_ExplosionEnergy_01" _returnvalue_2))
      (:`2`
        (`NiagaraFunctionLibrary.SpawnSystemAtLocation` "/Game/VFX/Stylized_VFX_StPack/VR/VR_Particles/P_VR_ExplosionEnergy_02.P_VR_ExplosionEnergy_02" _returnvalue_2))
      (:`3`
        (`NiagaraFunctionLibrary.SpawnSystemAtLocation` "/Game/VFX/Stylized_VFX_StPack/VR/VR_Particles/P_VR_ExplosionEnergy_03.P_VR_ExplosionEnergy_03" _returnvalue_2)))
    (`self.Again`)
    (else
      (switch `int` (`self.Level`)
        (:`1`
          (`NiagaraFunctionLibrary.SpawnSystemAtLocation` "/Game/VFX/Stylized_VFX_StPack/VR/VR_Particles/P_VR_ExplosionEffect_01.P_VR_ExplosionEffect_01" _returnvalue))
        (:`2`
          (`NiagaraFunctionLibrary.SpawnSystemAtLocation` "/Game/VFX/Stylized_VFX_StPack/VR/VR_Particles/P_VR_ExplosionEffect_02.P_VR_ExplosionEffect_02" _returnvalue))
        (:`3`
          (`NiagaraFunctionLibrary.SpawnSystemAtLocation` "/Game/VFX/Stylized_VFX_StPack/VR/VR_Particles/P_VR_ExplosionEffect_03.P_VR_ExplosionEffect_03" _returnvalue)))
      (`self.Again`))))

(event `self.ReceiveBeginPlay`
  (`KismetSystemLibrary.Delay` (+ (* (`self.Level`) 1.0) (* (`self.Variant`) 3.0)))
  (goto _label))

(fn `UserConstructionScript`)