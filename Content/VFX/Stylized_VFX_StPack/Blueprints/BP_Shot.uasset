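; BP_Shot is an actor that repeatedly plays one of three Niagara shot effects at its location, chosen by its Level value.
; BeginPlay staggers the first shot with a delay scaled by Level, then spawns the matching system.
; Each spawn passes the actor's forward vector to the User.Orientation parameter, then calls the Again event, which loops the spawn after a fixed delay.
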(event `Again`
  (bind _returnvalue (`self.K2_GetActorLocation`))
  (`KismetSystemLibrary.Delay` 3.0)
  (switch `int` (`self.Level`) :!label _label
    (:`1`
      (bind _returnvalue_2 (`NiagaraFunctionLibrary.SpawnSystemAtLocation` "/Game/VFX/Stylized_VFX_StPack/Particles/P_Shot_01.P_Shot_01" _returnvalue))
      (set `self.Niagara` _returnvalue_2))
    (:`2`
      (bind _returnvalue_3 (`NiagaraFunctionLibrary.SpawnSystemAtLocation` "/Game/VFX/Stylized_VFX_StPack/Particles/P_Shot_02.P_Shot_02" _returnvalue))
      (set `self.Niagara` _returnvalue_3))
    (:`3`
      (bind _returnvalue_4 (`NiagaraFunctionLibrary.SpawnSystemAtLocation` "/Game/VFX/Stylized_VFX_StPack/Particles/P_Shot_03.P_Shot_03" _returnvalue))
      (set `self.Niagara` _returnvalue_4)))
  (`FXSystemComponent.SetVectorParameter` (`self.Niagara`) "User.Orientation" (`self.GetActorForwardVector`))
  (`self.Again`))

(event `self.ReceiveBeginPlay`
  (`KismetSystemLibrary.Delay` (* (`self.Level`) 1.0))
  (goto _label))

(fn `UserConstructionScript`)