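; Pickup item actor that shows a widget when the player's BP_ThirdPersonCharacter is close enough to interact.
; On BeginPlay it caches the player, hides the widget and starts a looping timer that yaws the widget to face the player's capsule.
; Collision volume overlaps with that player toggle the CanInteract flag and widget visibility; the graph contains no actual pickup logic.
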(event `self.ReceiveBeginPlay`
  (`|ExecutionSequence`
    (:`then_0`
      (bind _asbp_third_person_character (cast `/Game/ThirdPerson/Blueprints/BP_ThirdPersonCharacter` (`GameplayStatics.GetPlayerCharacter` 0)))
      (set `self.PlayerRef` _asbp_third_person_character)
      (`SceneComponent.SetVisibility` (`self.Widget`) false false))
    (:`then_1`
      (`KismetSystemLibrary.K2_SetTimerDelegate` (delegate `Spin`) 0.1 true))))

(event `Spin`
  (bind _widget (`self.Widget`))
  (bind (_returnvalue_roll _returnvalue_pitch _returnvalue_yaw) (`KismetMathLibrary.BreakRotator` (`KismetMathLibrary.FindLookAtRotation` (`SceneComponent.K2_GetComponentLocation` _widget) (`SceneComponent.K2_GetComponentLocation` (`Character.CapsuleComponent` (`self.PlayerRef`))))))
  (`SceneComponent.K2_SetWorldRotation` _widget (`KismetMathLibrary.MakeRotator` 0.0 0.0 _returnvalue_yaw) false false))

(event `self.CollisionVolume.OnComponentBeginOverlap`
  (params (OverlappedComponent :type "PrimitiveComponent Object Reference") (OtherActor :type "Actor Object Reference") (OtherComp :type "PrimitiveComponent Object Reference") (OtherBodyIndex :type Integer) (bFromSweep :type Boolean) (SweepResult :type "HitResult Structure (by ref)"))
  (if (== OtherActor (`self.PlayerRef`))
    (set `self.CanInteract?` true)
    (`SceneComponent.SetVisibility` (`self.Widget`) true false)))

(event `self.CollisionVolume.OnComponentEndOverlap`
  (params (OverlappedComponent :type "PrimitiveComponent Object Reference") (OtherActor :type "Actor Object Reference") (OtherComp :type "PrimitiveComponent Object Reference") (OtherBodyIndex :type Integer))
  (if (== OtherActor (`self.PlayerRef`))
    (set `self.CanInteract?` false)
    (`SceneComponent.SetVisibility` (`self.Widget`) false false)))

(fn `UserConstructionScript`)